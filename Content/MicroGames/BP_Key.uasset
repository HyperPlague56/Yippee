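; BP_Key is a pickup key that stays hidden and non-collidable until no BC_MovingTarget actors remain in the level.
; Tick polls for targets, using the index returned by an array Add as the emptiness test, and drives visibility and collision.
; When the key first appears, a DoOnce plays an emitter and explosion sound.
; Player overlap then sets HaveKey on BP_FirstPersonCharacter, plays a sound and destroys the key.
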(event `self.ReceiveBeginPlay`
  ;[0.3113 0.5838 0.7969] PlayerAccess - Key Setup
  (bind _asbp_first_person_character (cast `/Game/FirstPerson/Blueprints/BP_FirstPersonCharacter` (`GameplayStatics.GetPlayerCharacter` 0)))
  (set `self.As BP First Person Character` _asbp_first_person_character))

(event `self.ReceiveTick`
  (params (DeltaSeconds :type "Float (single-precision)"))
  (bind _returnvalue (`SceneComponent.K2_GetComponentLocation` (`self.keyYay`)))
  ;[0.3088 0.7865 0.5399] Key Visibility
  (bind _outactors (`GameplayStatics.GetAllActorsOfClass` "/Game/MicroGames/BC_MovingTarget.BC_MovingTarget_C"))
  (bind _returnvalue_2 (`KismetArrayLibrary.Array_Add` _outactors))
  (bind _output_get (set `self.allTargetsGone` (<= _returnvalue_2 0)))
  (`SceneComponent.SetVisibility` (`self.keyYay`) _output_get true)
  (`self.SetActorEnableCollision` _output_get)
  ;[0 0.01855 1] Key Appearance Effects :}
  (if (`self.allTargetsGone`)
    (`/Engine/EditorBlueprintResources/StandardMacros.DoOnce` false
      (:`Completed`
        (`GameplayStatics.SpawnEmitterAtLocation` null _returnvalue)
        (`GameplayStatics.PlaySoundAtLocation` "/Game/StarterContent/Audio/Explosion02.Explosion02" _returnvalue (struct) 1.0 1.0 0.0 null null null null)))))

(event `self.keyCollider.OnComponentBeginOverlap`
  (params (OverlappedComponent :type "PrimitiveComponent Object Reference") (OtherActor :type "Actor Object Reference") (OtherComp :type "PrimitiveComponent Object Reference") (OtherBodyIndex :type Integer) (bFromSweep :type Boolean) (SweepResult :type "HitResult Structure (by ref)"))
  ;[1 0.6198 0.1014] Key Got!
  (if (and (== OtherActor (`self.As BP First Person Character`)) (`self.allTargetsGone`))
    (set `/Game/FirstPerson/Blueprints/BP_FirstPersonCharacter.haveKey?` true (`self.As BP First Person Character`))
    (`GameplayStatics.PlaySoundAtLocation` "/Game/StarterContent/Audio/Starter_Music01.Starter_Music01" (`self.K2_GetActorLocation`) (struct) 1.0 1.0 0.0 null null null null)
    (`self.K2_DestroyActor`)))

(fn `UserConstructionScript`)